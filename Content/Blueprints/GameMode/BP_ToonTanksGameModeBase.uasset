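; BP_ToonTanksGameModeBase is the Toon Tanks game mode Blueprint that handles the start and end of a round.
; StartGame creates the start-game widget and adds it to the viewport.
; GameOver shows the end-game widget with win or loss text chosen by its WonGame flag, then reopens the current level by name after a short delay.
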(event EventBeginPlay)

(event EventTick
  (params (DeltaSeconds :type Float%20%28single-precision%29)))

(event EventStartGame
  (bind _returnvalue (UserInterface|CreateWidget "/Game/Blueprints/Widgets/WBP_StartGameWIdget.WBP_StartGameWIdget_C"))
  (UserInterface|Viewport|AddtoViewport _returnvalue 0))

(event EventGameOver
  (params (WonGame :type Boolean))
  (bind _returnvalue (UserInterface|CreateWidget "/Game/Blueprints/Widgets/WBP_EndGameWIdget.WBP_EndGameWIdget_C"))
  (UserInterface|Viewport|AddtoViewport _returnvalue 0)
  (Variables|/Script/UMG.TextBlock|SetText (Variables|/Game/Blueprints/Widgets/WBP_EndGameWIdget.WBP_EndGameWIdget_C|GetDisplayText _returnvalue) (select WonGame "You Won!!!" "You Lost!"))
  (bind _returnvalue_2 (Game|GetCurrentLevelName true))
  (Utilities|FlowControl|Delay 2.0)
  (Game|OpenLevel(byName) (Utilities|String|StringToName _returnvalue_2)))

(fn ConstructionScript)